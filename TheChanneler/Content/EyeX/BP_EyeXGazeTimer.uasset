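; Actor component that sets up gaze dwell timing for an EyeX eye-tracking actor and flags when the player's gaze rests on it.
; BeginPlay applies the focus delay to the owner's dwell time and registers both with the Channeler HUD's timer lists.
; Tick sets PreGazeEvent from gaze hit and range, deactivating on gaze focus and optionally re-arming on look-away.
; Older ray-cast and HUD-drawing logic remains disconnected.
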(event Custom|ResetPreviousEyeXActor_Event
  (Utilities|FlowControl|Delay 2.0)
  (bind _asbp_the_channeler_hud (Utilities|Casting|CastToBP_TheChannelerHUD (HUD|GetHUD (Game|GetPlayerController 0))))
  (Variables|/Game/GameMode/BP_TheChannelerHUD.BP_TheChannelerHUD_C|SetPreviousEyeXActor _asbp_the_channeler_hud (Variables|Default|GetNewVar_0))
  (Development|PrintString ">>>>>>>>>>>>>>>>>>>>>>>>>>>>>>>>>>>>>>>>>>>>>>>>>>>>>>>>>>>>>>>>>>>>>>>>>>>>>>>>>>>>>>>>>>>>>>>>>>>>>>>>>>>>>"))

(event EventBeginPlay
  (bind _aseye_xactor_base (Utilities|Casting|CastToEyeXActorBase (Components|GetOwner)))
  (bind _output_get (Variables|Default|SetParentEyeX _aseye_xactor_base))
  (Variables|/Script/TobiiEyeX.EyeXActorBase|SetDwellTimeDeactivate _output_get 0.0)
  (Variables|/Script/TobiiEyeX.EyeXActorBase|SetDwellTimeActivate _output_get (Variables|Default|GetDelayGazeFocus))
  (Variables|Default|SetActiveDistance (Variables|/Script/TobiiEyeX.EyeXActorBase|GetMaxDistance _output_get))
  (bind _asbp_the_channeler_hud (Utilities|Casting|CastToBP_TheChannelerHUD (HUD|GetHUD (Game|GetPlayerController 0))))
  (Utilities|Array|AddUnique (Variables|/Game/GameMode/BP_TheChannelerHUD.BP_TheChannelerHUD_C|GetTimerEyeXActors _asbp_the_channeler_hud) _output_get)
  (Utilities|Array|AddUnique (Variables|/Game/GameMode/BP_TheChannelerHUD.BP_TheChannelerHUD_C|GetOriginalDwellTimesForTimers _asbp_the_channeler_hud) (Variables|Default|GetDelayGazeFocus)))

(event EventTick
  (params (DeltaSeconds :type Float%20%28single-precision%29))
  (bind _returnvalue (Game|GetPlayerController 0))
  (bind _returnvalue_2 (Pawn|GetControlledPawn _returnvalue))
  (if (Variables|Default|GetAcitve)
    (bind _aschanneler (Utilities|Casting|CastToChanneler _returnvalue_2 :!label _label))
    (bind _aseye_xplayer_controller (Utilities|Casting|CastToEyeXPlayerController (Game|GetPlayerController 0)))
    (Variables|Default|SetPre_GazeEvent (Math|Boolean|ANDBoolean (Variables|/Game/Blueprints/Characters/Channeler.Channeler_C|GetWasObjectHit _aschanneler) (== (.HitActor (Class|EyeXPlayerController|GetGazeHitResult _aseye_xplayer_controller)) (Components|GetOwner)) (<= (Transformation|GetHorizontalDistanceTo (stale EventBeginPlay _output_get) _returnvalue_2) (Variables|Default|GetActiveDistance)) (Variables|Default|GetAcitve) true))
    ;[1 1 1] deactivate once shrinked but still llooking
    (if (Class|EyeXActorBase|HasGazeFocus (Variables|Default|GetParentEyeX))
      (bind _output_get (Variables|Default|SetAcitve false))
      (else
        (Variables|Default|SetAcitve true)))
    (else
      (Utilities|FlowControl|Sequence
        (:then_0
          (goto _label))
        (:then_1
          ;[1 1 1] handle the regaze
          (if (not (Class|EyeXActorBase|HasGazeFocus (Variables|Default|GetParentEyeX)))
            (if (Variables|Default|GetShrinkOnRegaze)
              (Variables|Default|SetAcitve true))))))))

(fn SetIsEnabled
  (params (isEnabled :type Boolean))
  (Components|Activation|SetActive isEnabled false))