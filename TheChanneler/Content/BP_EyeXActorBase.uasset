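; Base actor for EyeX objects, with a trigger sphere sized from EyeXTriggerRadius at construction and an optional highlight mesh.
; On BeginPlay, a highlightable actor copies the visible mesh's static mesh onto HighlightMesh.
; SetHighlightVisibility toggles that duplicate mesh, or prints a message when the actor is not highlightable.
; SetEyeXVisibility is an empty stub.
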(event EventBeginPlay
  (if (and (Variables|Default|GetisHighlightable) (!= (Variables|Default|GetVisibleMesh) 0))
    (Components|StaticMesh|SetStaticMesh (Variables|Default|GetHighlightMesh) (Variables|/Script/Engine.StaticMeshComponent|GetStaticMesh (Variables|Default|GetVisibleMesh)))))

(event EventActorBeginOverlap
  (params (OtherActor :type Actor%20Object%20Reference)))

(event EventTick
  (params (DeltaSeconds :type Float%20%28single-precision%29)))

(fn ConstructionScript
  (Components|Sphere|SetSphereRadius (Variables|Default|GetSphere) (Variables|Default|GetEyeXTriggerRadius) true))

(fn SetEyeXVisibility
  (params (isVisible :type Boolean))
  (if isVisible
    _))

(fn SetHighlightVisibility
  (params (isHighlighted :type Boolean))
  (if (Variables|Default|GetisHighlightable)
    (Rendering|SetVisibility (Variables|Default|GetHighlightMesh) isHighlighted false)
    (else
      (Development|PrintString "EyeX Actor is not Highlightable"))))