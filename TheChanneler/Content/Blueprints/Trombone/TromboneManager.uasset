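; Trombone camera effect manager that moves the player's first-person camera to a trombone actor's target camera and back.
; StartEffect disables movement and look, then Tick lerps location, rotation and FOV over a frame count derived from distance and TransitionSpeed.
; After a timed wait, EnableReturnTrip swaps start and target for the return, and EndEffect restores controls.
; Frustum-height dolly-zoom math exists in UpdateTrombone but never runs, leaving plain FOV interpolation.
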(event EventBeginPlay
  (bind _aschanneler (Utilities|Casting|CastToChanneler (Pawn|GetControlledPawn (Game|GetPlayerController 0))))
  (Variables|Trombone|SetStartCamera (Variables|/Script/TheChanneler.FP_FirstPersonCharacter|GetFirstPersonCameraComponent _aschanneler)))

(event EventTick
  (params (DeltaSeconds :type Float%20%28single-precision%29))
  (bind _startcamera (Variables|Trombone|GetStartCamera))
  (if (Variables|Trombone|GetActive)
    (if (<= (Variables|Trombone|GetCurFrameCount) (Variables|Trombone|GetTotalFrameCount))
      (bind _output_get (Variables|Trombone|SetInterp (/ (Math|Conversions|ToFloat(Integer) (Variables|Trombone|GetCurFrameCount)) (Math|Conversions|ToFloat(Integer) (Variables|Trombone|GetTotalFrameCount)))))
      (Transformation|SetWorldLocation _startcamera (Math|Vector|Lerp(Vector) (Variables|Trombone|GetInitPosition) (Variables|Trombone|GetTargetLocation) _output_get) false true)
      (Transformation|SetWorldRotation _startcamera (Math|Rotator|Lerp(Rotator) (Variables|Trombone|GetInitRotation) (Variables|Trombone|GetTargetRotation) _output_get true) false false)
      (Variables|/Script/Engine.CameraComponent|SetFieldOfView _startcamera (Math|Float|Lerp (Variables|Trombone|GetInitFOV) (Variables|Default|GetTargetFOV) _output_get))
      (Math|Integer|IncrementInt (Variables|Trombone|GetCurFrameCount))
      (elif (Variables|Trombone|GetReturnTrip)
        (CallFunction|EndEffect)
        (else
          (Variables|Trombone|SetActive false)
          (Default|CallTromboneReachedTarget)
          (bind _returnvalue (Utilities|Time|SetTimerbyFunctionName 0 "EnableReturnTrip" (Variables|Default|GetWaitTIme)))
          (Variables|Default|SetTimerHandle _returnvalue))))))

(fn ConstructionScript)

(fn EnableTromboneEffect
  (params (enable :type Boolean))
  (Variables|Trombone|SetEnabled enable))

(fn RegisterTromboneActor
  (params (trombone :type Trombone%20Component%20Object%20Reference))
  (Utilities|Array|AddUnique (Variables|Trombone|GetAllTromboneActors) trombone))

(fn StartEffect
  (params (TromboneRef :type Trombone%20Component%20Object%20Reference))
  (if (Variables|Trombone|GetEnabled)
    (Variables|Trombone|SetWasEnabled (Variables|Trombone|GetEnabled))
    (Variables|Trombone|SetEnabled false)
    (Variables|Trombone|SetActive true)
    (bind _aschanneler_character (Utilities|Casting|CastToChannelerCharacter (Pawn|GetControlledPawn (Game|GetPlayerController 0))))
    (Variables|Trombone|SetWasMovementEnabled (Class|ChannelerCharacter|IsMovementEnabled _aschanneler_character))
    (Variables|Trombone|SetWasLookEnabled (Class|ChannelerCharacter|IsLookEnabled _aschanneler_character))
    (Class|ChannelerCharacter|DisableMovement _aschanneler_character)
    (Class|ChannelerCharacter|DisableLook _aschanneler_character)
    (Variables|Default|SetWaitTIme (Variables|/Game/Blueprints/Trombone/TromboneComponent.TromboneComponent_C|GetWaitTime TromboneRef))
    (Variables|Trombone|SetInitFOV (Variables|/Script/Engine.CameraComponent|GetFieldOfView (Variables|Trombone|GetStartCamera)))
    (CallFunction|Init (Variables|/Game/Blueprints/Trombone/TromboneComponent.TromboneComponent_C|GetTargetCamera TromboneRef))
    (Default|CallTromboneEffectStarted)))

(fn FrustrumHeightatDistance
  (params (Disatance :type Float%20%28single-precision%29) (Camera :type Camera%20Component%20Object%20Reference))
  (return (* (Math|Trig|Tan(Radians) (Math|Trig|DegreesToRadians (* (Variables|/Script/Engine.CameraComponent|GetFieldOfView Camera) 0.5))) (* Disatance 2.0))))

(fn Init
  (params (TargetCam :type Camera%20Component%20Object%20Reference))
  (bind _startcamera (Variables|Trombone|GetStartCamera))
  (Variables|Default|SetTargetFOV (Variables|/Script/Engine.CameraComponent|GetFieldOfView TargetCam))
  (bind _initheightatdist (CallFunction|FrustrumHeightatDistance (Math|Vector|VectorLength (- (Transformation|GetWorldLocation (Variables|Trombone|GetStartCamera)) (Transformation|GetWorldLocation TargetCam))) TargetCam))
  (Variables|Trombone|SetInitialHeigtAtDist _initheightatdist)
  (Variables|Trombone|SetInitPosition (Transformation|GetWorldLocation _startcamera))
  (Variables|Trombone|SetInitRotation (Transformation|GetWorldRotation _startcamera))
  (Variables|Trombone|SetTargetLocation (Transformation|GetWorldLocation TargetCam))
  (Variables|Trombone|SetTargetRotation (Transformation|GetWorldRotation TargetCam))
  (Variables|Trombone|SetCurFrameCount 0)
  (Variables|Trombone|SetTotalFrameCount (Math|Float|Truncate (/ (Math|Vector|VectorLength (- (Variables|Trombone|GetTargetLocation) (Variables|Trombone|GetInitPosition))) (Variables|Trombone|GetTransitionSpeed))))
  (Variables|Trombone|SetReturnTrip false))

(fn IsEffectOngoing
  (return (Variables|Trombone|GetActive)))

(fn IsEnabled
  (return (Variables|Trombone|GetEnabled)))

(fn EndEffect
  (bind _startcamera (Variables|Trombone|GetStartCamera))
  (bind _aschanneler_character (Utilities|Casting|CastToChannelerCharacter (Pawn|GetControlledPawn (Game|GetPlayerController 0))))
  (Utilities|FlowControl|Sequence
    (:then_0
      (if (Variables|Trombone|GetWasMovementEnabled)
        (Class|ChannelerCharacter|EnableMovement _aschanneler_character)))
    (:then_1
      (if (Variables|Trombone|GetWasLookEnabled)
        (Class|ChannelerCharacter|EnableLook _aschanneler_character)))
    (:then_2
      (Variables|Trombone|SetActive false)
      (Variables|Trombone|SetEnabled (Variables|Trombone|GetWasEnabled))
      (Transformation|SetWorldLocationAndRotation _startcamera (Variables|Trombone|GetTargetLocation) (Variables|Trombone|GetTargetRotation) false true)
      (Variables|/Script/Engine.CameraComponent|SetFieldOfView _startcamera (Variables|Default|GetTargetFOV))
      (Default|CallTromboneEnded))))

(fn EnableReturnTrip
  (Class|KismetSystemLibrary|ClearTimerHandle (Variables|Default|GetTimerHandle))
  (Default|CallTromboneReturning)
  (Variables|Trombone|SetReturnTrip true)
  (Variables|Trombone|SetCurFrameCount 0)
  (Variables|Trombone|SetTempPosition (Variables|Trombone|GetInitPosition))
  (Variables|Trombone|SetInitPosition (Variables|Trombone|GetTargetLocation))
  (Variables|Trombone|SetTargetLocation (Variables|Trombone|GetTempPosition))
  (Variables|Trombone|SetTempRotation (Variables|Trombone|GetInitRotation))
  (Variables|Trombone|SetInitRotation (Variables|Trombone|GetTargetRotation))
  (Variables|Trombone|SetTargetRotation (Variables|Trombone|GetTempRotation))
  (Variables|Default|SetTempFOV (Variables|Trombone|GetInitFOV))
  (Variables|Trombone|SetInitFOV (Variables|Default|GetTargetFOV))
  (Variables|Default|SetTargetFOV (Variables|Default|GetTempFOV))
  (Variables|Trombone|SetActive true))

(fn TromboneFOV
  (params (Height :type Float%20%28single-precision%29) (Distance :type Float%20%28single-precision%29))
  (return (Math|Trig|RadiansToDegrees (* (Math|Trig|Atan(Degrees) (/ (* Height 0.5) Distance)) 2.0))))

(fn UpdateTrombone
  (bind _initialheigtatdist (Variables|Trombone|GetInitialHeigtAtDist))
  (bind _startcamera (Variables|Trombone|GetStartCamera))
  (if (Variables|Trombone|GetReturnTrip)
    (bind _fov (CallFunction|TromboneFOV _initialheigtatdist (Math|Vector|VectorLength (- (Variables|Trombone|GetInitPosition) (Transformation|GetWorldLocation (Variables|Trombone|GetStartCamera))))))
    (bind _output_get (Variables|/Script/Engine.CameraComponent|SetFieldOfView _startcamera (Math|Float|Clamp(Float) _fov 5.0 1.7e+02)))
    (Development|PrintString (Utilities|String|ToString(Float) _output_get))
    (else
      (bind _fov_2 (CallFunction|TromboneFOV _initialheigtatdist (Math|Vector|VectorLength (- (Variables|Trombone|GetTargetLocation) (Transformation|GetWorldLocation (Variables|Trombone|GetStartCamera))))))
      (Variables|/Script/Engine.CameraComponent|SetFieldOfView _startcamera (Math|Float|Clamp(Float) _fov_2 5.0 1.7e+02))
      (Development|PrintString (Utilities|String|ToString(Float) (Math|Float|Clamp(Float) _fov_2 5.0 1.7e+02))))))