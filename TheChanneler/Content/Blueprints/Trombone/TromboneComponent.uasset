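; Actor component that triggers a "trombone" effect when its owning actor receives EyeX eye-tracking gaze focus.
; On BeginPlay it requires an EyeXCollisionActor owner, binds to its gaze-focus event and caches the owner's first camera as the target.
; Gaze focus passes the component to a trombone manager's StartEffect, using a reference this graph never sets.
; Debug prints flag an invalid owner, a missing camera and each focus event.
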(event Custom|OnOwnerGotGazeFocus
  (Development|PrintString "Hello")
  (Default|StartEffect (Variables|Default|GetTromboneMangerRef) self))

(event EventBeginPlay
  (bind _returnvalue (Components|GetOwner))
  (bind _returnvalue_2 (Actor|GetComponentsByClass _returnvalue "/Script/Engine.CameraComponent"))
  (bind _aseye_xcollision_actor (Utilities|Casting|CastToEyeXCollisionActor _returnvalue)
    (:then
      (EventDispatchers|BindEventtoOnGazeFocus _aseye_xcollision_actor (delegate Custom|OnOwnerGotGazeFocus))
      (if (> (Utilities|Array|Length _returnvalue_2) 0)
        (Variables|Default|SetTargetCamera (Utilities|Array|Get(acopy) _returnvalue_2))
        (else
          (Development|PrintString "Trombone Component owner must have a camera component" true true "(R=1.000000,G=0.035352,B=0.000000,A=1.000000)"))))
    (:CastFailed
      (Development|PrintString "Owner of TromboneComponent needs to be an EyeXCollisionActor" true true "(R=1.000000,G=0.000000,B=0.000000,A=1.000000)"))))

(event EventTick
  (params (DeltaSeconds :type Float%20%28single-precision%29)))