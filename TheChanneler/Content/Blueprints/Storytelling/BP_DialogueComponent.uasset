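; Widget component that displays NPC dialogue on an in-world DialogueWidget, with configurable font size, box color and horizontal flip.
; Showing dialogue turns off the HUD gaze and hiding it restores it, while optional looping timers drive a skippable typewriter reveal and yaw/pitch billboarding toward the camera.
; A separate event shows timed one-off lines, such as market hawker barks, independently of the Storytelling API.
; Tick contains leftover debug printing.
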(event Custom|DisplayOneOffDialogue
  (params (Time :type Float%20%28single-precision%29) (Text :type String))
  (bind _returnvalue (Utilities|Text|ToText(String) Text))
  (bind _dialoguewidgetref (Variables|Default|GetDialogueWidgetRef))
  (bind _dialoguetext (Variables|/Game/Blueprints/Storytelling/DialogueWidget.DialogueWidget_C|GetDialogueText _dialoguewidgetref))
  ;[1 1 1] Displays Dialogue without reference to Storytelling API. Used for one off instances, like Hawkers in the market
  (Rendering|Components|TextRender|SetText _dialoguetext _returnvalue)
  (Widget|SetVisibility _dialoguewidgetref "Visible")
  (Utilities|FlowControl|Delay Time)
  (if (Utilities|Enum|Equal(Enum) (Class|TextBlock|GetText _dialoguetext) _returnvalue)
    (Widget|SetVisibility _dialoguewidgetref "Hidden")
    (Rendering|Components|TextRender|SetText _dialoguetext "")))

(event EventBeginPlay
  (bind _returnvalue (UserInterface|GetUserWidgetObject))
  (bind _asdialogue_widget (Utilities|Casting|CastToDialogueWidget _returnvalue)
    (:then
      (Variables|Default|SetDialogueWidgetRef _asdialogue_widget)
      (CallFunction|UpdateFontSize (Variables|Default|GetFontSize))
      (Default|SetDialogueBoxColor _asdialogue_widget (Variables|Default|GetImageColor))
      (Variables|Default|SetWidgetForText _asdialogue_widget))
    (:CastFailed
      _))
  (Widget|SetVisibility _returnvalue "Hidden")
  (if (Variables|Default|GetisFlipped)
    (Widget|Transform|SetRenderScale (Variables|/Game/Blueprints/Storytelling/DialogueWidget.DialogueWidget_C|GetTextBoxImage (Variables|Default|GetWidgetForText)) "(X=-1.000000,Y=1.000000)")))

(event EventSkipAnimation
  ;[0 0 0] SkipAnimation
  (Class|KismetSystemLibrary|ClearTimerHandle (Variables|Default|GetAnimateTextTimerHandle))
  (Variables|Default|SetbIsAnimating false)
  (Rendering|Components|TextRender|SetText (Variables|/Game/Blueprints/Storytelling/DialogueWidget.DialogueWidget_C|GetDialogueText (Variables|Default|GetDialogueWidgetRef)) (Utilities|Text|ToText(String) (Variables|Default|GetDialogue))))

(event EventShowDialogue
  (bind _dialoguewidgetref (Variables|Default|GetDialogueWidgetRef))
  (bind _asbp_the_channeler_hud (Utilities|Casting|CastToBP_TheChannelerHUD (HUD|GetHUD (Game|GetPlayerController 0)))
    (:then
      ;[0 0 0] ShowDialpgue
      (Class|TheChannelerHUD|TurnOffGaze _asbp_the_channeler_hud))
    (:CastFailed
      (Development|PrintString "Cast to ChannelerHud failed")))
  (Widget|SetVisibility _dialoguewidgetref "Visible")
  (if (Variables|Default|GetAnimate)
    (Variables|Default|SetTextindex 1)
    (bind _returnvalue (Utilities|Time|SetTimerbyFunctionName 0 "AnimateText" (Utilities|Struct|BreakTextAnimation (Variables|Default|GetAnimationProperties)) true))
    (Variables|Default|SetAnimateTextTimerHandle _returnvalue)
    (Rendering|Components|TextRender|SetText (Variables|/Game/Blueprints/Storytelling/DialogueWidget.DialogueWidget_C|GetDialogueText (Variables|Default|GetDialogueWidgetRef)) "")
    (Variables|Default|SetbIsAnimating true)
    (else
      (Default|SetDialogue _dialoguewidgetref (Variables|Default|GetDialogue))))
  (if (Variables|Default|GetisBillBoard)
    (bind _returnvalue_2 (Utilities|Time|SetTimerbyFunctionName 0 "BillBoardWidget" 0.01 true))))

(event EventHideDialogue
  (bind _asbp_the_channeler_hud (Utilities|Casting|CastToBP_TheChannelerHUD (HUD|GetHUD (Game|GetPlayerController 0))))
  ;[0 0 0] HideDialogue
  (Class|TheChannelerHUD|TurnonGaze _asbp_the_channeler_hud)
  (Widget|SetVisibility (Variables|Default|GetDialogueWidgetRef) "Hidden")
  (Class|KismetSystemLibrary|ClearTimerHandle (stale EventShowDialogue _returnvalue_2)))

(event EventTick
  (params (DeltaSeconds :type Float%20%28single-precision%29))
  (bind _returnvalue (Components|GetOwner))
  (bind (_devicerotation _deviceposition) (Class|HeadMountedDisplayFunctionLibrary|GetOrientationandPosition))
  (bind _returnvalue_2 (Utilities|GetObjectName _returnvalue))
  (Development|PrintString _returnvalue_2)
  (if (Utilities|Enum|Equal(Enum) _returnvalue_2 "GhostlyShellNPC")
    (Development|PrintString (Utilities|String|Append (Utilities|String|ToString(Byte) (Widget|GetVisibility (Variables|Default|GetDialogueWidgetRef))) ", " (Utilities|String|ToString(Rotator) _devicerotation) ", " (Utilities|String|ToString(Vector) _deviceposition)))))

(fn BillboardWidget
  (bind _returnvalue (Game|GetPlayerCameraManager 0))
  (bind _returnvalue_2 (Transformation|GetWorldLocation))
  (bind _returnvalue_3 (Camera|GetCameraLocation _returnvalue))
  (bind _returnvalue_4 (Math|Rotator|FindLookatRotation _returnvalue_2 _returnvalue_3))
  (Utilities|IsValid _returnvalue
    (:Is%20Valid
      (Transformation|SetWorldRotation (Math|Rotator|MakeRotator 0.0 (.pitch _returnvalue_4) (.yaw _returnvalue_4)) false false))))

(fn UpdateFontSize
  (params (newFontSize :type Integer))
  (bind _dialoguewidgetref (Variables|Default|GetDialogueWidgetRef))
  (bind _dialoguetext (Variables|/Game/Blueprints/Storytelling/DialogueWidget.DialogueWidget_C|GetDialogueText _dialoguewidgetref))
  (bind _font (Variables|/Script/UMG.TextBlock|GetFont _dialoguetext))
  (bind (_fontobject _fontmaterial _typefacefontname) (Utilities|Struct|BreakSlateFontInfo _font))
  (Class|TextBlock|SetFont _dialoguetext (Utilities|Struct|MakeSlateFontInfo _fontobject _fontmaterial _typefacefontname newFontSize))
  (Variables|Default|SetCurrentFontSize newFontSize))

(fn AnimateText
  (Rendering|Components|TextRender|SetText (Variables|/Game/Blueprints/Storytelling/DialogueWidget.DialogueWidget_C|GetDialogueText (Variables|Default|GetDialogueWidgetRef)) (Utilities|Text|ToText(String) (Utilities|String|GetSubstring (Variables|Default|GetDialogue) 0 (Variables|Default|GetTextindex))))
  (if (>= (Variables|Default|GetTextindex) (Utilities|String|Len (Variables|Default|GetDialogue)))
    (Class|KismetSystemLibrary|ClearTimerHandle (Variables|Default|GetAnimateTextTimerHandle))
    (Variables|Default|SetbIsAnimating false)
    (else
      (Math|Integer|IncrementInt (Variables|Default|GetTextindex)))))