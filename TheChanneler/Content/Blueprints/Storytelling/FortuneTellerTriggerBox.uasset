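; A trigger box that makes a linked fortune teller NPC call out for help when the player walks in.
; On BeginPlay it moves its audio component to the NPC's location and assigns the configured sound.
; While active, a player overlap shows a one-off dialogue line on the NPC, plays the sound and switches the NPC's animation for the set duration before changing it again.
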(event EventBeginPlay
  (Transformation|SetWorldLocation (Variables|Default|GetChannelerAudio) (Transformation|GetWorldLocation (Variables|/Game/Blueprints/Characters/BlobGhostBase.BlobGhostBase_C|GetRoot (Variables|Default|GetNPC))) false false)
  (Audio|Components|Audio|SetSound (Variables|Default|GetChannelerAudio) (Variables|Default|GetNPCSoundToPlay)))

(event EventActorBeginOverlap
  (params (OtherActor :type Actor%20Object%20Reference))
  (bind _npc (Variables|Default|GetNPC))
  (if (and (== OtherActor (Game|GetPlayerCharacter 0)) (Variables|Default|GetisActive))
    (Default|DisplayOneOffDialogue (Variables|/Game/Blueprints/Puzzles/LockPick/FortuneTellerNPC.FortuneTellerNPC_C|GetBP_DialogueComponent (Variables|Default|GetNPC)) (Variables|Default|GetDuration) "Hey, can you help me please?")
    (Audio|Components|Audio|Play (Variables|Default|GetChannelerAudio) 0.0)
    (Default|SetAnimation _npc "NewEnumerator3")
    (Utilities|FlowControl|Delay (Variables|Default|GetDuration))
    (Default|SetAnimation _npc "NewEnumerator13")))

(event EventTick
  (params (DeltaSeconds :type Float%20%28single-precision%29)))

(fn ConstructionScript)