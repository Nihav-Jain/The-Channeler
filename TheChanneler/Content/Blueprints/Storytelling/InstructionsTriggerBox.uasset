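; InstructionsTriggerBox is a trigger volume that shows an in-game instructions widget while the player character is inside it.
; It creates the InGameInstructions widget on BeginPlay, then adds it to the viewport and plays its Fade animation on overlap.
; On exit it plays the fade in reverse, waits briefly, then removes the widget, using state flags to keep it if the player has re-entered.
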(event OnComponentEndOverlap(CollisionComponent)
  (params (OtherActor :type Actor%20Object%20Reference) (OtherComp :type Primitive%20Component%20Object%20Reference) (OtherBodyIndex :type Integer))
  (bind _instructionswidget (Variables|Default|GetInstructionsWidget))
  ;[1 1 1] Fade down instructions widget and remove it from the screen if the player is not currently in the collision box
  (if (== OtherActor (Game|GetPlayerCharacter 0))
    (Variables|Default|SetisInTrigger false)
    (UserInterface|Animation|PlayAnimation _instructionswidget (Variables|/Game/Blueprints/Storytelling/InGameInstructions.InGameInstructions_C|GetFade _instructionswidget) 0.0 1 "Reverse")
    (Utilities|FlowControl|Delay 2.0)
    (if (not (and (Variables|Default|GetisInTrigger) (Variables|Default|GetisOnScreen)))
      (Widget|RemovefromParent _instructionswidget)
      (Variables|Default|SetisOnScreen false))))

(event EventBeginPlay
  (bind _returnvalue (UserInterface|CreateWidget "/Game/Blueprints/Storytelling/InGameInstructions.InGameInstructions_C" (Game|GetPlayerController 0)))
  (Variables|Default|SetInstructionsWidget _returnvalue))

(event EventActorBeginOverlap
  (params (OtherActor :type Actor%20Object%20Reference))
  (bind _instructionswidget (Variables|Default|GetInstructionsWidget))
  ;[1 1 1] Add Instructions Widget to Screen and fade it up!
  (if (== OtherActor (Game|GetPlayerCharacter 0))
    (Variables|Default|SetisInTrigger true)
    (if (Variables|Default|GetisOnScreen)
      _
      (else
        (UserInterface|Viewport|AddtoViewport _instructionswidget 0)
        (Variables|Default|SetisOnScreen true)))
    (UserInterface|Animation|PlayAnimation _instructionswidget (Variables|/Game/Blueprints/Storytelling/InGameInstructions.InGameInstructions_C|GetFade _instructionswidget) 0.0 1 "Forward")))

(fn ConstructionScript)