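; StorytellerActor is an actor that drives story dialogue through its StoryDialogueManager.
; On BeginPlay it binds story-ended and story-parsed callbacks and passes the manager to SetStoryManager; Tick updates the manager each frame.
; Releasing the NextDialogue input advances to the next node, and story end only prints a message, while the parsed callback is empty.
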(event Custom|StoryEnded
  (Development|PrintString "Story ended"))

(event Custom|StoryParsed)

(event EventTick
  (params (DeltaSeconds :type Float%20%28single-precision%29))
  (Class|StoryDialogueManager|Update (Variables|Default|GetStoryDialogueManager) DeltaSeconds))

(event EventBeginPlay
  (bind _storydialoguemanager (Variables|Default|GetStoryDialogueManager))
  (EventDispatchers|BindEventtoStoryEnded _storydialoguemanager (delegate Custom|StoryEnded))
  (EventDispatchers|BindEventtoStoryParsed _storydialoguemanager (delegate Custom|StoryParsed))
  (Class|ChannelerUtils|SetStoryManager _storydialoguemanager))

(event Input|ActionEvents|InputActionNextDialogue
  (params (Key :type Key%20Structure :default "AnyKey"))
  (:Released
    (Class|StoryManager|GotoNextNode (Variables|Default|GetStoryDialogueManager))))

(fn ConstructionScript)