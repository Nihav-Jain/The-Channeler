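; An actor Blueprint that switches the evil ghost's animation in time with the "resurrect" story dialogue.
; On BeginPlay it takes the first StorytellerActor and waits for its StoryDialogueManager to finish parsing the story.
; It then looks up the "resurrect" node by name and binds to its dialogue start and end events, each setting a different animation state on EvilGhost.
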(event Custom|StoryParsed
  ;[1 1 1] Resurrect
  (bind _asstory_dialogue_node (Utilities|Casting|CastToStoryDialogueNode (Class|StoryManager|GetNodebyName (Variables|/Game/Blueprints/Storytelling/StorytellerActor.StorytellerActor_C|GetStoryDialogueManager (Variables|Default|GetStoryDialogueActor)) "resurrect")))
  (EventDispatchers|BindEventtoDialogueStarted _asstory_dialogue_node (delegate Custom|ResurrectStart))
  ;[1 1 1] End Resurrect
  (EventDispatchers|BindEventtoDialogueEnded _asstory_dialogue_node (delegate Custom|ResurrectEnd)))

(event Custom|ResurrectEnd
  ;[1 1 1] End Resurrect
  (Default|SetAnimation (Variables|Default|GetEvilGhost) "NewEnumerator0"))

(event Custom|ResurrectStart
  ;[1 1 1] Resurrect
  (Default|SetAnimation (Variables|Default|GetEvilGhost) "NewEnumerator15"))

(event EventBeginPlay
  (bind _outactors (Actor|GetAllActorsOfClass "/Game/Blueprints/Storytelling/StorytellerActor.StorytellerActor_C"))
  (bind _output_get (Variables|Default|SetStoryDialogueActor (Utilities|Array|Get(acopy) _outactors)))
  (EventDispatchers|BindEventtoStoryParsed (Variables|/Game/Blueprints/Storytelling/StorytellerActor.StorytellerActor_C|GetStoryDialogueManager _output_get) (delegate Custom|StoryParsed)))

(event EventActorBeginOverlap
  (params (OtherActor :type Actor%20Object%20Reference)))

(event EventTick
  (params (DeltaSeconds :type Float%20%28single-precision%29)))

(fn ConstructionScript)