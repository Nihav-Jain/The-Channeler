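; Game instance for Channeler that holds checkpoint, playtest and audio state across levels.
; Init loads or creates the save and restores the latest checkpoint; Shutdown writes it back and deactivates analytics.
; Helpers control heat map recording, apply SFX, voice and music volumes, and toggle between Main and StartMap in playtest builds.
; Puzzle completion flags can trigger a playtest survey URL, though the older level-sequence logic is disconnected.
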(event Custom|EventSetVolume
  ;[1 1 1] setting the audio after start map
  (CallFunction|SetVolume))

(event EventInit
  ;[1 1 0] USE FOR SETTING PLAYTEST VARIABLES!
  (Variables|Default|SetPlaytestBuild true)
  (Variables|Default|SetUsePlaytest1Levels true)
  ;[0.2 0.06667 0] Load / Create Save Game State on Game Initialization
  (bind _returnvalue (SaveGame|DoesSaveGameExist (Variables|Default|GetSaveSlotName) (Variables|Default|GetSaveUserID)))
  (if _returnvalue
    (bind _returnvalue_2 (SaveGame|LoadGamefromSlot (Variables|Default|GetSaveSlotName) (Variables|Default|GetSaveUserID)))
    (bind _aschanneler_save_instance (Utilities|Casting|CastToChannelerSaveInstance _returnvalue_2)
      (:then
        (bind _output_get (Variables|Default|SetChannelerSaveGameInstance _aschanneler_save_instance))
        (Variables|Default|SetCurrentCheckpoint (Variables|/Game/Blueprints/CheckpointSystem/ChannelerSaveInstance.ChannelerSaveInstance_C|GetLatestCheckpoint _output_get)))
      (:CastFailed
        (Development|PrintString "Init Cast FAILED!!!" :!label _label)))
    (else
      (bind _returnvalue_3 (SaveGame|CreateSaveGameObject "/Game/Blueprints/CheckpointSystem/ChannelerSaveInstance.ChannelerSaveInstance_C"))
      (bind _aschanneler_save_instance_2 (Utilities|Casting|CastToChannelerSaveInstance _returnvalue_3)
        (:then
          (Variables|Default|SetChannelerSaveGameInstance _aschanneler_save_instance_2))
        (:CastFailed
          (goto _label))))))

(event EventShutdown
  (bind _channelersavegameinstance (Variables|Default|GetChannelerSaveGameInstance))
  ;[0.2 0.06667 0] Save the Latest Game State on Game Termination
  (Variables|/Game/Blueprints/CheckpointSystem/ChannelerSaveInstance.ChannelerSaveInstance_C|SetLatestCheckpoint _channelersavegameinstance (Variables|Default|GetCurrentCheckpoint))
  (SaveGame|SaveGametoSlot _channelersavegameinstance (Variables|Default|GetSaveSlotName) (Variables|Default|GetSaveUserID))
  ;[0.2 0.06667 0] Stop and Save any Heat Map Recording
  (Development|PrintString "VLOG: Saving HeatMap to File" false true "(R=1.000000,G=0.533333,B=0.000000,A=1.000000)")
  (Class|Analytics|DeactivateAllModules (Variables|Default|GetAnalytics)))

(fn StartHeatMap
  (Class|Analytics|ActivateModule (Variables|Default|GetAnalytics) "/Script/TheChanneler.HeatMap")
  (Utilities|IsHeatMapRecording
    (:False
      (Development|PrintString "VLOG: Error, Not Activating!" true true "(R=1.000000,G=0.503778,B=0.055860,A=1.000000)"))
    (:IsNull
      (Development|PrintString "VLOG: Error, Heat Map Is Not Created"))))

(fn StopHeatMap
  (Class|Analytics|DeactivateModule (Variables|Default|GetAnalytics) "/Script/TheChanneler.HeatMap")
  (Utilities|IsHeatMapRecording
    (:True
      (Development|PrintString "VLOG: Error, Still Active!" true true "(R=1.000000,G=0.503778,B=0.055860,A=1.000000)"))
    (:IsNull
      (Development|PrintString "VLOG: Error, Heat Map Is Not Created"))))

(fn OpenURL
  (if (Variables|Default|GetPlaytestBuild)
    (if (Variables|Default|GetUsePlaytest1Levels)
      (Variables|Default|SetURL "https://docs.google.com/forms/d/164629RP_QZKMbVHQtPH2Muc-A0JeoHpZuC8t5WNAbLQ/viewform?entry.496938770=")
      (else
        (Variables|Default|SetURL "https://docs.google.com/forms/d/1spl2gHNayeDNsYtu0wFsm-F0C9x1paFl9Q9ltDar41g/viewform?entry.879856204="))))
  (Utilities|Platform|LaunchURL (Utilities|String|Append (Variables|Default|GetURL) (Variables|Default|GetUserName)))
  (Game|OpenLevel(byName) "StartMap"))

(fn CheckifAllPuzzlesCompleted
  (if (Math|Boolean|ANDBoolean (Variables|Default|GetisPeripheralDone) (Variables|Default|GetisRLGLDone) (Variables|Default|GetisTromboneDone) (Variables|Default|GetisPickPocketDone) (Variables|Default|GetisGhostlyShellDone) (Variables|Default|GetisClutteredRoomDone) (Variables|Default|GetisWeepingStatueDone) (Variables|Default|GetisAfterImageDone) (Variables|Default|GetisFocalPointDone) (Variables|Default|GetisWallOfEyesDone))
    (CallFunction|OpenURL)
    (Variables|Default|SetisPeripheralDone false)
    (Variables|Default|SetisRLGLDone false)
    (Variables|Default|SetisTromboneDone false)
    (Variables|Default|SetisWallOfEyesDone false)
    (Variables|Default|SetisFocalPointDone false)
    (Variables|Default|SetisAfterImageDone false)
    (Variables|Default|SetisPickPocketDone false)
    (Variables|Default|SetisGhostlyShellDone false)
    (Variables|Default|SetisWeepingStatueDone false)
    (Variables|Default|SetisClutteredRoomDone false)
    (else
      (Game|OpenLevel(byName) "ProxyArtWalkThrough"))))

(fn OpenNextLevel
  (if (Variables|Default|GetPlaytestBuild)
    (bind _returnvalue (Game|GetCurrentLevelName true))
    (if (Utilities|Enum|Equal(Enum) _returnvalue "Main")
      (Game|OpenLevel(byName) "StartMap")
      (else
        (Game|OpenLevel(byName) "Main")))))

(fn SetLevelCompleted
  (switch Utilities|FlowControl|Switch|SwitchonLevelNames (Variables|Default|GetCurrentLevel)
    (:NewEnumerator0
      (Variables|Default|SetisAfterImageDone true))
    (:NewEnumerator1
      (Variables|Default|SetisClutteredRoomDone true))
    (:NewEnumerator2
      (Variables|Default|SetisFocalPointDone true))
    (:NewEnumerator3
      (Variables|Default|SetisGhostlyShellDone true))
    (:NewEnumerator4
      (Variables|Default|SetisPeripheralDone true))
    (:NewEnumerator5
      (Variables|Default|SetisPickPocketDone true))
    (:NewEnumerator6
      (Variables|Default|SetisRLGLDone true))
    (:NewEnumerator7
      (Variables|Default|SetisTromboneDone true))
    (:NewEnumerator8
      (Variables|Default|SetisWallOfEyesDone true))
    (:NewEnumerator9
      (Variables|Default|SetisWeepingStatueDone true))))

(fn OpenGoogleForm
  (Utilities|Platform|LaunchURL (Variables|Default|GetURL)))

(fn ChangeVolumebyChannel
  (params (Channel :type Array%20of%20Channeler%20Audio%20Component%20Object%20References) (NewVolumeMultiplier :type Float%20%28single-precision%29))
  (for _array_element Channel
    (Audio|Components|Audio|SetVolumeMultiplier _array_element NewVolumeMultiplier :!class /Script/Engine.AudioComponent)))

(fn SetVolume
  (CallFunction|ChangeVolumebyChannel (Variables|Default|GetChannelerSFXAudioComponentArray) (Variables|GUI|GetGlobalSFXVolume))
  (CallFunction|ChangeVolumebyChannel (Variables|Default|GetChannelerVoiceAudioComponentArray) (Variables|GUI|GetGlobalVoiceVolume))
  (CallFunction|ChangeVolumebyChannel (Variables|Default|GetChannelerMusicAudioComponentArray) (Variables|GUI|GetGlobalMusicVolume)))