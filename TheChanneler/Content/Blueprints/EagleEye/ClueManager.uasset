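; Clue manager that records which clues the player has found and presents each discovery.
; ClueFound pauses the game through the Channeler, then plays that clue's animation on the game mode's current ClueMenu widget.
; Clues two and four also move Bucket Head through the BucketHeadGateManager; after a delay, each new clue joins the found list.
; The YouFoundAClue popup is created at BeginPlay, but its timed display logic is disconnected.
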(event Custom|DisplayClueFound
  (params (ClueNumber :type EClueNumber%20Enum))
  (bind _returnvalue (Math|Conversions|ToInteger(Byte) ClueNumber))
  (bind _cluestatelist (Variables|Default|GetClueStateList))
  (bind _aschanneler (Utilities|Casting|CastToChanneler (Game|GetPlayerCharacter 0)))
  (Default|PauseGame _aschanneler)
  (bind _asthe_channeler_game_mode (Utilities|Casting|CastToTheChannelerGameMode (Game|GetGameMode))
    (:then
      (bind _returnvalue_2 (Class|TheChannelerGameMode|GetCurrentMenuWidget _asthe_channeler_game_mode))
      (bind _asclue_menu (Utilities|Casting|CastToClueMenu _returnvalue_2)))
    (:CastFailed
      _))
  (switch Utilities|FlowControl|Switch|SwitchonEClueNumber ClueNumber
    (:NewEnumerator0
      (UserInterface|Animation|PlayAnimation _asclue_menu (Variables|/Game/GameMode/ClueMenu.ClueMenu_C|GetClue1Found _asclue_menu) 0.0 1 "Forward"))
    (:NewEnumerator1
      (UserInterface|Animation|PlayAnimation _asclue_menu (Variables|/Game/GameMode/ClueMenu.ClueMenu_C|GetClue2Found _asclue_menu) 0.0 1 "Forward")
      (Default|MoveBucketHeadAway (Variables|Default|GetBucketHeadManager)))
    (:NewEnumerator2
      (UserInterface|Animation|PlayAnimation _asclue_menu (Variables|/Game/GameMode/ClueMenu.ClueMenu_C|GetClue3Found _asclue_menu) 0.0 1 "Forward"))
    (:NewEnumerator3
      (UserInterface|Animation|PlayAnimation _asclue_menu (Variables|/Game/GameMode/ClueMenu.ClueMenu_C|GetClue4Found _asclue_menu) 0.0 1 "Forward")
      (Default|MovetoStatues (Variables|Default|GetBucketHeadManager))))
  (Utilities|FlowControl|Delay 2.0)
  (if (>= _returnvalue 0)
    (if (< _returnvalue (Utilities|Array|Length _cluestatelist))
      (if (not (Utilities|Array|Get(acopy) _cluestatelist _returnvalue))
        (Utilities|Array|SetArrayElem _cluestatelist _returnvalue true)
        (Utilities|Array|Add (Variables|Default|GetCluesFoundList) ClueNumber)))))

(event Custom|RemoveClueFoundDisplay
  (Widget|RemovefromParent (Variables|Default|GetWidgetRef))
  (Class|KismetSystemLibrary|ClearTimerHandle))

(event EventBeginPlay
  (bind _returnvalue (|GetNumEnumEntries))
  (bind _cluestatelist (Variables|Default|GetClueStateList))
  (bind _returnvalue_2 (UserInterface|CreateWidget "/Game/Blueprints/EagleEye/YouFoundAClue.YouFoundAClue_C" (Game|GetPlayerController 0)))
  (Variables|Default|SetWidgetRef _returnvalue_2)
  (Utilities|Array|Resize _cluestatelist _returnvalue)
  (for _index (range 0 (- _returnvalue 1))
    (Utilities|Array|SetArrayElem _cluestatelist _index false))
  (bind _outactors (Actor|GetAllActorsOfClass "/Game/Blueprints/Puzzles/BucketHeadAndClues/BucketHeadGateManager.BucketHeadGateManager_C"))
  (Variables|Default|SetBucketHeadManager (Utilities|Array|Get(acopy) _outactors)))

(event EventActorBeginOverlap
  (params (OtherActor :type Actor%20Object%20Reference)))

(event EventTick
  (params (DeltaSeconds :type Float%20%28single-precision%29)))

(fn ConstructionScript)

(fn ClueFound
  (params (Clue%20Number :type EClueNumber%20Enum))
  (CallFunction|DisplayClueFound Clue%20Number))

(fn GetCluesFound
  (return (Variables|Default|GetCluesFoundList)))

(fn GetTexture
  (params (ClueNumber :type EClueNumber%20Enum))
  (return (Utilities|Array|Get(acopy) (Variables|Default|GetClueImageList) (Math|Conversions|ToInteger(Byte) ClueNumber))))