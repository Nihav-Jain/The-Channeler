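; Eagle Eye volume that controls the highlighting of eagle eye objects as actors enter and leave it.
; On begin overlap, it registers itself as the active instance for the overlapping actor, then checks the player Channeler's eagle eye state.
; If eagle eye is enabled, group 1 lights alongside group 3 for left or group 2 for right, clearing the opposite group.
; End overlap zeroes all eagle eye material intensity.
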(event Collision|EventActorBeginOverlap
  (params (OtherActor :type Actor%20Object%20Reference))
  (Class|EagleEyeUtil|SetActiveInstance OtherActor self)
  (bind _aschanneler (Utilities|Casting|CastToChanneler (Game|GetPlayerCharacter 0)))
  (if (Class|ChannelerCharacter|IsEagleEyeEnabled _aschanneler)
    ;[1 1 1] Highlight eagle eye objects when re-entering a volume with eagle eye active
    (if (Class|ChannelerCharacter|IsLeftEagleEyeActive _aschanneler)
      (CallFunction|SetEagleEyeInsensity 0.0 2.0)
      (CallFunction|SetEagleEyeInsensity 1.0 3.0)
      (CallFunction|SetEagleEyeInsensity 1.0 1.0)
      (elif (Class|ChannelerCharacter|IsRightEagleEyeActive _aschanneler)
        (CallFunction|SetEagleEyeInsensity 0.0 3.0)
        (CallFunction|SetEagleEyeInsensity 1.0 2.0)
        (CallFunction|SetEagleEyeInsensity 1.0 1.0)))))

(event Collision|EventActorEndOverlap
  (params (OtherActor :type Actor%20Object%20Reference))
  (Class|EagleEyeVolume|SetAllEagleEyeMaterialIntensity 0.0 -1.0))

(fn ConstructionScript)