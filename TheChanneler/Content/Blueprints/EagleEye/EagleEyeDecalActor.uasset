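; Decal actor that shows its decal only while the player's Eagle Eye ability is active.
; On BeginPlay it caches the player character as a Channeler.
; Tick polls the Channeler's Eagle Eye state and toggles decal visibility through two DoOnce gates that reset each other, so visibility is set only when the state changes.
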(event EventBeginPlay
  (bind _aschanneler (Utilities|Casting|CastToChanneler (Game|GetPlayerCharacter 0)))
  (Variables|Default|SetChanneler _aschanneler))

(event EventTick
  (params (DeltaSeconds :type Float%20%28single-precision%29))
  (if (Class|ChannelerCharacter|IsEagleEyeActive (Variables|Default|GetChanneler))
    (Utilities|FlowControl|DoOnce false :!label _label
      (:Completed
        (Rendering|SetVisibility (Variables|Decal|GetDecal) true false)
        (goto _label_2 Reset)))
    (else
      (Utilities|FlowControl|DoOnce false :!label _label_2
        (:Completed
          (Rendering|SetVisibility (Variables|Decal|GetDecal) false false)
          (goto _label Reset))))))

(fn ConstructionScript)