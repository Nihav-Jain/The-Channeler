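; Decoy object for the Channeler's Eagle Eye mode that tells the player there is nothing of interest when gazed at.
; If Eagle Eye is active on gaze focus, it plays a wrong-object sound and hint once, hides its ectoplasm decal, destroys that decal's box and shuts off its EyeX gaze timer.
; BeginPlay disables the timer, and the Tick logic that toggled it with Eagle Eye is disconnected.
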(event EventTick
  (params (DeltaSeconds :type Float%20%28single-precision%29)))

(event EventBeginPlay
  (bind _aschanneler (Utilities|Casting|CastToChanneler (Game|GetPlayerCharacter 0)))
  (Variables|Default|SetChannelerCharacter _aschanneler)
  (Default|SetIsEnabled (Variables|Default|GetBP_EyeXGazeTimer) false))

(event EventGotGazeFocusBP
  (bind _ectoplasmdecalreference (Variables|Default|GetEctoplasmDecalReference))
  (bind _channeleraudio (Variables|Default|GetChannelerAudio))
  (bind _bp_eyexgazetimer (Variables|Default|GetBP_EyeXGazeTimer))
  (bind _aschanneler (Utilities|Casting|CastToChanneler (Game|GetPlayerCharacter 0)))
  (if (Default|IsEagleEyeActive _aschanneler)
    (Utilities|FlowControl|DoOnce false
      (:Completed
        (Default|SetIsEnabled (Variables|Default|GetBP_EyeXGazeTimer) false)
        (Audio|Components|Audio|SetSound _channeleraudio "/Game/Sound/WrongObjectSound.WrongObjectSound")
        (Audio|Components|Audio|Play _channeleraudio 0.0)
        (bind _outactors (Actor|GetAllActorsOfClass "/Game/Blueprints/Characters/Channeler.Channeler_C"))
        (bind _hint_manager (Default|GetHintManager (Utilities|Array|Get(acopy) _outactors)))
        (Default|DisplayHint _hint_manager "There's nothing of interest here." 3.0 true)
        (Rendering|SetActorHiddenInGame _ectoplasmdecalreference true)
        (Components|DestroyComponent (Variables|/Game/Blueprints/EagleEye/EagleEyeDecalActor.EagleEyeDecalActor_C|GetBox _ectoplasmdecalreference))
        (Actor|Tick|SetActorTickEnabled false)
        (Variables|/Game/EyeX/BP_EyeXGazeTimer.BP_EyeXGazeTimer_C|SetAcitve _bp_eyexgazetimer false)
        (Default|SetIsEnabled _bp_eyexgazetimer false)
        (Components|Activation|Deactivate _bp_eyexgazetimer)))))

(fn ConstructionScript)