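; EagleEyeCorrectObject is the correct gaze target for a numbered clue in the eye-tracked Eagle Eye mechanic.
; Gaining gaze focus while the Channeler's Eagle Eye is active plays a completion sound, then reports the clue to the game mode's ClueManager after a delay.
; It then disables itself and matching wrong objects, hides matching decals, and ends the analytics duration event.
; The Tick logic toggling the gaze timer is disconnected.
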(event EventTick
  (params (DeltaSeconds :type Float%20%28single-precision%29)))

(event EventBeginPlay
  (bind _aschanneler (Utilities|Casting|CastToChanneler (Game|GetPlayerCharacter 0)))
  (Variables|Default|SetChannelerCharacter _aschanneler)
  (Default|SetIsEnabled (Variables|Default|GetBP_EyeXGazeTimer) false))

(event EventGotGazeFocusBP
  (bind _bp_eyexgazetimer (Variables|Default|GetBP_EyeXGazeTimer))
  (bind _channeleraudio (Variables|Default|GetChannelerAudio))
  (bind _aschanneler (Utilities|Casting|CastToChanneler (Game|GetPlayerCharacter 0)))
  (if (Class|ChannelerCharacter|IsEagleEyeActive _aschanneler)
    (Utilities|FlowControl|DoOnce false
      (:Completed
        (Default|SetIsEnabled (Variables|Default|GetBP_EyeXGazeTimer) false)
        (Audio|Components|Audio|SetSound _channeleraudio "/Game/Sound/GazeComplete.GazeComplete")
        (Audio|Components|Audio|Play _channeleraudio 0.0)
        (Utilities|FlowControl|Delay 1.25) ; Delay so sound plays before menu pops up
        ;[1 1 1] Clue Found!
        (Development|PrintString "You Found a Clue!")
        (bind _aseye_xmenu_game_mode (Utilities|Casting|CastToEyeXMenuGameMode (Game|GetGameMode)))
        (Default|ClueFound (Variables|/Game/GameMode/EyeXMenuGameMode.EyeXMenuGameMode_C|GetClueManager _aseye_xmenu_game_mode) (Variables|Default|GetClueNumber))
        (bind _outactors (Actor|GetAllActorsOfClass "/Game/Blueprints/EagleEye/EagleEyeWrongObject.EagleEyeWrongObject_C"))
        (for _array_element _outactors
          ;[1 1 1] Disable interaction
          (if (Utilities|Enum|Equal(Enum) (Variables|/Game/Blueprints/EagleEye/EagleEyeWrongObject.EagleEyeWrongObject_C|GetClueNumber _array_element) (Variables|Default|GetClueNumber))
            (Actor|Tick|SetActorTickEnabled _array_element)
            (Variables|/Game/EyeX/BP_EyeXGazeTimer.BP_EyeXGazeTimer_C|SetAcitve (Variables|/Game/Blueprints/EagleEye/EagleEyeWrongObject.EagleEyeWrongObject_C|GetBP_EyeXGazeTimer _array_element) false)
            (Default|SetIsEnabled (Variables|/Game/Blueprints/EagleEye/EagleEyeWrongObject.EagleEyeWrongObject_C|GetBP_EyeXGazeTimer _array_element) false)
            (Components|Activation|Deactivate (Variables|/Game/Blueprints/EagleEye/EagleEyeWrongObject.EagleEyeWrongObject_C|GetBP_EyeXGazeTimer _array_element))))
        ;[1 1 1] Hide decals
        (bind _outactors_2 (Actor|GetAllActorsOfClass "/Game/Blueprints/EagleEye/EagleEyeDecalActor.EagleEyeDecalActor_C"))
        (for _array_element_2 _outactors_2
          (if (Utilities|Enum|Equal(Enum) (Variables|/Game/Blueprints/EagleEye/EagleEyeDecalActor.EagleEyeDecalActor_C|GetClueNumber _array_element_2) (Variables|Default|GetClueNumber))
            (Rendering|SetVisibility (Variables|/Script/Engine.DecalActor|GetDecal _array_element_2) false false)
            (Actor|Tick|SetActorTickEnabled _array_element_2)))
        ;[1 1 1] Deactivate self
        (Actor|Tick|SetActorTickEnabled false)
        (Variables|/Game/EyeX/BP_EyeXGazeTimer.BP_EyeXGazeTimer_C|SetAcitve _bp_eyexgazetimer false)
        (Default|SetIsEnabled _bp_eyexgazetimer false)
        (Components|Activation|Deactivate _bp_eyexgazetimer)
        ;[1 1 1] End Duration Logger
        (Utilities|FlowControl|DoOnce false
          (:Completed
            (bind _returnvalue (Class|ChannelerUtils|GetChannelerAnalytics))
            (bind _asduration_logger (Utilities|Casting|CastToDurationLogger (Class|Analytics|GetAnalyticsModule _returnvalue "/Script/TheChanneler.DurationLogger")))
            (Class|DurationLogger|EndEventTime _asduration_logger (Utilities|String|Append (Utilities|String|MakeLiteralString "Finding Clue: ") (Utilities|GetObjectName self)))))))))

(fn ConstructionScript)