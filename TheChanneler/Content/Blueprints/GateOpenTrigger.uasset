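; Gaze-activated trigger that opens a linked gate when it receives Tobii EyeX gaze focus.
; Gaining focus also plays audio, hides the visible mesh, disables collision on its meshes and the one-shot dialogue trigger.
; A DoOnce then jumps the story dialogue to scene 04 and disables the distraction puzzle's freeze cam.
; Tick keeps the gaze timer disabled because its condition is hardcoded false, leaving the Channeler's eagle-eye check unused.
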(event EventTick
  (params (DeltaSeconds :type Float%20%28single-precision%29))
  (bind _bp_eyexgazetimer (Variables|Default|GetBP_EyeXGazeTimer))
  (bind _aschanneler (Utilities|Casting|CastToChanneler (Game|GetPlayerCharacter 0)))
  (if false
    (Default|SetIsEnabled _bp_eyexgazetimer true)
    (else
      (Default|SetIsEnabled _bp_eyexgazetimer false))))

(event EventBeginPlay
  (bind _outactors (Actor|GetAllActorsOfClass "/Game/Blueprints/Storytelling/StorytellerActor.StorytellerActor_C"))
  (Variables|Default|SetStoryDialogueReference (Utilities|Array|Get(acopy) _outactors)))

(event EventActorBeginOverlap
  (params (OtherActor :type Actor%20Object%20Reference)))

(event EventGotGazeFocusBP
  (bind _visiblemesh (Variables|Default|GetVisibleMesh))
  (Development|PrintString "Got Gaze")
  (Default|OpenGate (Variables|Default|GetGate))
  (Audio|Components|Audio|Play (Variables|Default|GetChannelerAudio) 0.0)
  (Rendering|SetVisibility _visiblemesh false false)
  (Collision|SetCollisionEnabled _visiblemesh "NoCollision")
  (Collision|SetActorEnableCollision (Variables|Default|GetOneShotDialogueTrigger) false)
  (Utilities|FlowControl|DoOnce false
    (:Completed
      (bind _asstory_jump_node (Utilities|Casting|CastToStoryJumpNode (Class|StoryManager|GetNodebyName (Variables|/Game/Blueprints/Storytelling/StorytellerActor.StorytellerActor_C|GetStoryDialogueManager (Variables|Default|GetStoryDialogueReference)) "jumpToScene04")))
      (Class|StoryJumpNode|JumptoNode _asstory_jump_node)
      (Class|Puzzle|DisableMyFreezeCam (Variables|Default|GetDistractionPuzzleReference)))))

(event EventLostGazeFocusBP
  (Development|PrintString "Lost Gaze"))

(fn ConstructionScript)

(fn DestroySelf
  (bind _visiblemesh (Variables|Default|GetVisibleMesh))
  (Development|SetHiddeninGame _visiblemesh true false)
  (Rendering|SetVisibility _visiblemesh false false)
  (Collision|SetCollisionEnabled _visiblemesh "NoCollision")
  (Collision|SetCollisionEnabled (Variables|Default|GetHiddenMesh) "NoCollision"))