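; Sparks effect actor that emits intermittent bursts from a particle system while its InPuzzle flag is set.
; The construction script assigns the particle template from a variable, and the effect starts with zeroed emission.
; Tick counts down a randomized timer, then raises radius and spawn parameters for a few random seconds before zeroing them and re-rolling the timer.
; AdjustParticleSystem clamps and writes those float parameters to the particle system.
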(event EventBeginPlay
  (Variables|Default|SetTimer (Math|Random|RandomFloatinRange 15.0 4e+01))
  (CallFunction|AdjustParticleSystem 0.0 0.0 0.0))

(event EventActorBeginOverlap
  (params (OtherActor :type Actor%20Object%20Reference)))

(event EventTick
  (params (DeltaSeconds :type Float%20%28single-precision%29))
  (if (Variables|Default|GetInPuzzle)
    (if (not (Variables|Default|GetisActive))
      (bind _output_get (Variables|Default|SetTimer (- (Variables|Default|GetTimer) DeltaSeconds)))
      (if (<= _output_get 0.0)
        (Variables|Default|SetisActive true)
        (CallFunction|AdjustParticleSystem 5.0 1e+01 1e+02)
        (Utilities|FlowControl|Delay (Math|Random|RandomFloatinRange 4.0 8.0))
        (CallFunction|AdjustParticleSystem 0.0 0.0 0.0)
        (Variables|Default|SetTimer (Math|Random|RandomFloatinRange 2e+01 3e+01))
        (Variables|Default|SetisActive false)))))

(fn ConstructionScript
  (Effects|Components|ParticleSystem|SetTemplate (Variables|Default|GetParticleSystem) (Variables|Default|GetParticleSystemVar)))

(fn AdjustParticleSystem
  (params (Radius :type Float%20%28single-precision%29) (CenterSpawn :type Float%20%28single-precision%29) (OutsideSpawn :type Float%20%28single-precision%29))
  (bind _particlesystem (Variables|Default|GetParticleSystem))
  (Effects|Components|ParticleSystem|SetFloatParameter _particlesystem "Radius" (Math|Float|Clamp(Float) Radius 0.0 5.0))
  (Effects|Components|ParticleSystem|SetFloatParameter _particlesystem "CenterSpawn" (Math|Float|Clamp(Float) CenterSpawn 0.0 5e+01))
  (Effects|Components|ParticleSystem|SetFloatParameter _particlesystem "OutsideSpawn" (Math|Float|Clamp(Float) OutsideSpawn 0.0 1e+02)))