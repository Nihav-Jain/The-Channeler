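; MusicTrigger is an overlap-triggered actor that changes the music when the player enters it.
; On BeginPlay it assigns its SoundFadeIn clip to ChannelerAudio1.
; When the player character begins overlapping, it passes that clip to the referenced theme manager's TransitionMusic with a fixed fade duration.
; End overlap does nothing, and a fade-out on the manager's ChannelerAudio is left disconnected.
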(event EventBeginPlay
  (Audio|Components|Audio|SetSound (Variables|Default|GetChannelerAudio1) (Variables|Default|GetSoundFadeIn)))

(event EventActorBeginOverlap
  (params (OtherActor :type Actor%20Object%20Reference))
  (if (== OtherActor (Game|GetPlayerCharacter 0))
    (Default|TransitionMusic (Variables|Default|GetThemeManagerReference) (Variables|Default|GetSoundFadeIn) 2.0)))

(event Collision|EventActorEndOverlap
  (params (OtherActor :type Actor%20Object%20Reference)))

(fn ConstructionScript)