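; Music manager actor that switches level themes in response to story dialogue and ghost chases.
; TransitionMusic crossfades between two audio components, loading the requested clip onto the idle channel and tracking the active one.
; Once the StorytellerActor's story parses, named dialogue nodes trigger character themes on start or restore the market theme on end.
; Chase music uses a timer to hand its intro off to a loop just before it finishes.
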(event Custom|EndTutorial
  (CallFunction|TransitionMusic (Variables|Default|GetMainMarketTheme) 1.0))

(event Custom|PlayShellTheme
  (CallFunction|TransitionMusic (Variables|Default|GetShellTheme) 1.0))

(event Custom|PlayBucketTheme
  (CallFunction|TransitionMusic (Variables|Default|GetBucketTheme) 1.0))

(event Custom|PlayBucketHead2
  (CallFunction|TransitionMusic (Variables|Default|GetBucketTheme) 1.0))

(event Custom|StoryParsed
  (Utilities|FlowControl|Sequence
    (:then_0
      (bind _asstory_dialogue_node (Utilities|Casting|CastToStoryDialogueNode (Class|StoryManager|GetNodebyName (Variables|/Game/Blueprints/Storytelling/StorytellerActor.StorytellerActor_C|GetStoryDialogueManager (Variables|Default|GetStoryTellerAPI)) "ShellDialogue")))
      (EventDispatchers|BindEventtoDialogueStarted _asstory_dialogue_node (delegate Custom|PlayShellTheme)))
    (:then_1
      (bind _asstory_dialogue_node_2 (Utilities|Casting|CastToStoryDialogueNode (Class|StoryManager|GetNodebyName (Variables|/Game/Blueprints/Storytelling/StorytellerActor.StorytellerActor_C|GetStoryDialogueManager (Variables|Default|GetStoryTellerAPI)) "BucketHeadDialogue")))
      (EventDispatchers|BindEventtoDialogueStarted _asstory_dialogue_node_2 (delegate Custom|PlayBucketTheme)))
    (:then_2
      (bind _asstory_dialogue_node_3 (Utilities|Casting|CastToStoryDialogueNode (Class|StoryManager|GetNodebyName (Variables|/Game/Blueprints/Storytelling/StorytellerActor.StorytellerActor_C|GetStoryDialogueManager (Variables|Default|GetStoryTellerAPI)) "BucketHeadDialogue2")))
      (EventDispatchers|BindEventtoDialogueStarted _asstory_dialogue_node_3 (delegate Custom|PlayBucketHead2)))
    (:then_3
      (bind _asstory_dialogue_node_4 (Utilities|Casting|CastToStoryDialogueNode (Class|StoryManager|GetNodebyName (Variables|/Game/Blueprints/Storytelling/StorytellerActor.StorytellerActor_C|GetStoryDialogueManager (Variables|Default|GetStoryTellerAPI)) "MotherDialogue")))
      (EventDispatchers|BindEventtoDialogueStarted _asstory_dialogue_node_4 (delegate Custom|PlayMotherDialogue)))
    (:then_4
      (bind _asstory_dialogue_node_5 (Utilities|Casting|CastToStoryDialogueNode (Class|StoryManager|GetNodebyName (Variables|/Game/Blueprints/Storytelling/StorytellerActor.StorytellerActor_C|GetStoryDialogueManager (Variables|Default|GetStoryTellerAPI)) "EndMother")))
      (EventDispatchers|BindEventtoDialogueEnded _asstory_dialogue_node_5 (delegate Custom|EndMotherDialogue)))
    (:then_5
      (bind _asstory_dialogue_node_6 (Utilities|Casting|CastToStoryDialogueNode (Class|StoryManager|GetNodebyName (Variables|/Game/Blueprints/Storytelling/StorytellerActor.StorytellerActor_C|GetStoryDialogueManager (Variables|Default|GetStoryTellerAPI)) "EndBucket1")))
      (EventDispatchers|BindEventtoDialogueEnded _asstory_dialogue_node_6 (delegate Custom|EndBucket1)))
    (:then_6
      (bind _asstory_dialogue_node_7 (Utilities|Casting|CastToStoryDialogueNode (Class|StoryManager|GetNodebyName (Variables|/Game/Blueprints/Storytelling/StorytellerActor.StorytellerActor_C|GetStoryDialogueManager (Variables|Default|GetStoryTellerAPI)) "EndBucket2")))
      (EventDispatchers|BindEventtoDialogueEnded _asstory_dialogue_node_7 (delegate Custom|EndBucket2)))
    (:then_7
      (bind _asstory_dialogue_node_8 (Utilities|Casting|CastToStoryDialogueNode (Class|StoryManager|GetNodebyName (Variables|/Game/Blueprints/Storytelling/StorytellerActor.StorytellerActor_C|GetStoryDialogueManager (Variables|Default|GetStoryTellerAPI)) "ShowJournalMenu")))
      (EventDispatchers|BindEventtoDialogueEnded _asstory_dialogue_node_8 (delegate Custom|EndTutorial)))))

(event Custom|PlayMotherDialogue
  (CallFunction|TransitionMusic (Variables|Default|GetMotherTheme) 1.0))

(event Custom|EndMotherDialogue
  (CallFunction|TransitionMusic (Variables|Default|GetMainMarketTheme) 1.0))

(event Custom|EndBucket1
  (CallFunction|TransitionMusic (Variables|Default|GetMainMarketTheme) 1.0))

(event Custom|StartGhostChaseMusic
  (CallFunction|TransitionMusic (Variables|Default|GetGhostChaseStart) 1.0)
  (bind _returnvalue (Utilities|Time|SetTimerbyFunctionName 0 "ToLoopingGhostChase" (- (Variables|/Script/Engine.SoundBase|GetDuration (Variables|Default|GetGhostChaseStart)) 0.1)))
  (Variables|Default|SetStartScaryMusicHandle _returnvalue))

(event Custom|TransitionMusic
  (params (AudioClip :type Sound%20Wave%20Object%20Reference) (Fade%20Duration :type Float%20%28single-precision%29))
  (Utilities|IsValid AudioClip
    (:Is%20Valid
      (bind _assound_wave (Utilities|Casting|CastToSoundWave (Variables|/Script/Engine.AudioComponent|GetSound (Variables|Default|GetActiveAudioSource))))
      (if (not (== AudioClip _assound_wave))
        (if (== (Variables|Default|GetActiveAudioSource) (Variables|Default|GetChannelerAudio))
          (bind _assound_wave_2 (Utilities|Casting|CastToSoundWave (Variables|/Script/Engine.AudioComponent|GetSound (Variables|Default|GetChannelerAudio1))))
          (if (== _assound_wave_2 AudioClip)
            _
            (else
              (Audio|Components|Audio|SetSound (Variables|Default|GetChannelerAudio1) AudioClip)))
          (CallFunction|CrossFade (Variables|Default|GetChannelerAudio) (Variables|Default|GetChannelerAudio1) Fade%20Duration)
          (else
            (bind _assound_wave_3 (Utilities|Casting|CastToSoundWave (Variables|/Script/Engine.AudioComponent|GetSound (Variables|Default|GetChannelerAudio))))
            (if (== _assound_wave_3 AudioClip)
              _
              (else
                (Audio|Components|Audio|SetSound (Variables|Default|GetChannelerAudio) AudioClip)))
            (CallFunction|CrossFade (Variables|Default|GetChannelerAudio1) (Variables|Default|GetChannelerAudio) Fade%20Duration)))))))

(event Custom|EndBucket2
  (CallFunction|TransitionMusic (Variables|Default|GetMainMarketTheme) 1.0))

(event EventBeginPlay
  (bind _channeleraudio (Variables|Default|GetChannelerAudio))
  (bind _fadestrength (Variables|Default|GetFadeStrength))
  (Audio|Components|Audio|SetSound _channeleraudio (Variables|Default|GetMainMarketTheme))
  (Audio|Components|Audio|SetSound (Variables|Default|GetChannelerAudio1) (Variables|Default|GetBucketTheme))
  (Audio|Components|Audio|SetVolumeMultiplier (Variables|Default|GetChannelerAudio) _fadestrength :!class /Script/Engine.AudioComponent)
  (Audio|Components|Audio|SetVolumeMultiplier (Variables|Default|GetChannelerAudio1) _fadestrength :!class /Script/Engine.AudioComponent)
  (Audio|Components|Audio|Play _channeleraudio 0.0)
  (Variables|Default|SetActiveAudioSource (Variables|Default|GetChannelerAudio))
  (bind _outactors (Actor|GetAllActorsOfClass "/Game/Blueprints/Storytelling/StorytellerActor.StorytellerActor_C"))
  (bind _output_get (Variables|Default|SetStoryTellerAPI (Utilities|Array|Get(acopy) _outactors)))
  (EventDispatchers|BindEventtoStoryParsed (Variables|/Game/Blueprints/Storytelling/StorytellerActor.StorytellerActor_C|GetStoryDialogueManager _output_get) (delegate Custom|StoryParsed)))

(fn ConstructionScript)

(fn CrossFade
  (params (FadeOut :type Channeler%20Audio%20Component%20Object%20Reference) (FadeIn :type Channeler%20Audio%20Component%20Object%20Reference) (FadeDuration :type Float%20%28single-precision%29))
  (Class|ChannelerAudioComponent|FadeOutMute FadeOut FadeDuration 0.0)
  (Class|ChannelerAudioComponent|FadeinMute FadeIn FadeDuration (Variables|/Script/Engine.AudioComponent|GetVolumeMultiplier FadeIn) 0.0)
  (Variables|Default|SetActiveAudioSource FadeIn))

(fn FadeOutAudioComponents
  (Class|ChannelerAudioComponent|FadeOutMute (Variables|Default|GetChannelerAudio) 1.0 0.0)
  (Class|ChannelerAudioComponent|FadeOutMute (Variables|Default|GetChannelerAudio1) 1.0 0.0))

(fn PlayOneShot
  (params (SoundToPlay :type Sound%20Wave%20Object%20Reference))
  (bind _channeleraudio1 (Variables|Default|GetChannelerAudio1))
  (Class|ChannelerAudioComponent|FadeOutMute (Variables|Default|GetChannelerAudio) 1.0 0.0)
  (Audio|Components|Audio|SetSound _channeleraudio1 SoundToPlay)
  (bind _aschanneler_game_instance (Utilities|Casting|CastToChannelerGameInstance (Game|GetGameInstance)))
  (Class|ChannelerAudioComponent|FadeinMute _channeleraudio1 1.0 (Variables|/Game/Blueprints/CheckpointSystem/ChannelerGameInstance.ChannelerGameInstance_C|GetGlobalMusicVolume _aschanneler_game_instance) 0.0)
  (bind _aschanneler_game_instance_2 (Utilities|Casting|CastToChannelerGameInstance (Game|GetGameInstance)))
  (Default|SetVolume _aschanneler_game_instance_2))

(fn ToLoopingGhostChase
  (bind _assound_wave (Utilities|Casting|CastToSoundWave (Variables|/Script/Engine.AudioComponent|GetSound (Variables|Default|GetActiveAudioSource))))
  (if (== _assound_wave "/Game/Sound/Music/Ghost_Chase_Beginning.Ghost_Chase_Beginning")
    (CallFunction|TransitionMusic (Variables|Default|GetGhostChaseLoop) 0.01)
    (Class|KismetSystemLibrary|ClearTimerHandle (Variables|Default|GetStartScaryMusicHandle))
    (else
      (Class|KismetSystemLibrary|ClearTimerHandle (Variables|Default|GetStartScaryMusicHandle)))))