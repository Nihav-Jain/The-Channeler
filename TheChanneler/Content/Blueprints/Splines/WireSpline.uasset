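; WireSpline is a spline-based actor Blueprint, apparently an unfinished tool for building wires from spline meshes.
; Its construction script adds one spline mesh component per MeshAmount count, without setting their start or end points along the spline.
; An even-spacing distance calculation from the spline length exists but is unconnected, and the event graph holds only disabled default events.
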(event EventBeginPlay)

(event EventActorBeginOverlap
  (params (OtherActor :type Actor%20Object%20Reference)))

(event EventTick
  (params (DeltaSeconds :type Float%20%28single-precision%29)))

(fn ConstructionScript
  (bind _meshamount (Variables|Default|GetMeshAmount))
  (if (> _meshamount 0)
    (for _index (range 0 (- _meshamount 1))
      (AddComponent|AddSplineMeshComponent false))))