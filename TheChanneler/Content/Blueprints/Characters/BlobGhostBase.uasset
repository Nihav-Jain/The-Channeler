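; BlobGhostBase is a base Blueprint for a blob ghost character with configurable color, eye expression and animation.
; The construction script creates a dynamic material instance on the skeletal mesh and applies the ghost color, while eye masks swap a texture parameter by index.
; BeginPlay caches the Blob_Animation_v5 instances of the main and Culling meshes, and SetAnimation sends the same state change to both.
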(event EventBeginPlay
  (Utilities|FlowControl|Sequence
    (:then_0
      (bind _asblob_animation_v_5 (Utilities|Casting|CastToBlob_Animation_v5 (Components|SkeletalMesh|GetAnimInstance (Variables|Default|GetSkeletalMesh))))
      (Variables|Animations|SetGhostAnimation _asblob_animation_v_5))
    (:then_1
      (bind _asblob_animation_v_5_2 (Utilities|Casting|CastToBlob_Animation_v5 (Components|SkeletalMesh|GetAnimInstance (Variables|Default|GetCulling))))
      (Variables|Animations|SetCullingGhostAnimation _asblob_animation_v_5_2))))

(event EventActorBeginOverlap
  (params (OtherActor :type Actor%20Object%20Reference)))

(event EventTick
  (params (DeltaSeconds :type Float%20%28single-precision%29)))

(fn ConstructionScript
  (bind _returnvalue (Rendering|Material|CreateDynamicMaterialInstance (Variables|Default|GetSkeletalMesh) 0 (Variables|Default|GetMaterialToUse) :!class /Script/Engine.PrimitiveComponent))
  (Variables|Default|SetMaterial%20Instance _returnvalue)
  (CallFunction|SetGhostColor (Variables|Default|GetColor%20of%20Ghost)))

(fn SetEyeMask
  (params (EyeMask :type EyeMaskEnum%20Enum))
  (Rendering|Material|SetTextureParameterValue (Variables|Default|GetMaterial%20Instance) "EyeExpressionMask" (Utilities|Array|Get(acopy) (Variables|Default|GetEyeMaskTextures) (Math|Conversions|ToInteger(Byte) EyeMask))))

(fn SetGhostColor
  (params (Color :type Linear%20Color%20Structure))
  (Rendering|Material|SetVectorParameterValue (Variables|Default|GetMaterial%20Instance) "BlobColor" Color :!class /Script/Engine.MaterialInstanceDynamic))

(fn SetAnimation
  (params (Animation :type BlobGhostAnimEnum%20Enum))
  (Default|ChangeState (Variables|Animations|GetGhostAnimation) Animation))